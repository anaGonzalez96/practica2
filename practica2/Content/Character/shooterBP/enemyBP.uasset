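; Enemy character Blueprint that takes damage, dies for score and deals repeated melee-range damage to the hero.
; AffectHealth updates health and, on death, disables pawn and world-dynamic collision, adds 500 score to the Tecnocampus game mode, detaches the controller and destroys the actor after a delay.
; Hero overlap with DamageVolume starts a looping timer at the attack rate that damages the hero until the overlap ends.
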(event OnComponentBeginOverlap(DamageVolume)
  (params (OverlappedComponent :type Primitive%20Component%20Object%20Reference) (OtherActor :type Actor%20Object%20Reference) (OtherComp :type Primitive%20Component%20Object%20Reference) (OtherBodyIndex :type Integer) (bFromSweep :type Boolean) (SweepResult :type Hit%20Result%20Structure%20%28by%20ref%29))
  (bind _ashero_character (Utilities|Casting|CastToHeroCharacter OtherActor))
  (Variables|Default|Sethero _ashero_character)
  (Utilities|Time|SetTimerbyFunctionName 0 "DamageHero" (/ 1.0 (Variables|Default|GetattackPerSecond)) true))

(event OnComponentEndOverlap(DamageVolume)
  (params (OverlappedComponent :type Primitive%20Component%20Object%20Reference) (OtherActor :type Actor%20Object%20Reference) (OtherComp :type Primitive%20Component%20Object%20Reference) (OtherBodyIndex :type Integer))
  (if (== (Variables|Default|Gethero) OtherActor)
    (Utilities|Time|ClearTimerbyFunctionName 0 "DamageHero")))

(event Custom|DamageHero
  (Default|AffectHealth (Variables|Default|Gethero) (Variables|Default|GetDamagedone)))

(event EventAffectHealth
  (params (Value :type Float%20%28single-precision%29))
  (CallFunction|CalculateHealth Value)
  (Development|PrintString (Utilities|String|ToString(Float) (Variables|Default|Gethealth)))
  (if (Variables|Default|Getisdead)
    (Collision|SetCollisionResponsetoChannel (Variables|Default|GetCapsuleComponent) "ECC_WorldDynamic" "ECR_Ignore")
    (Collision|SetCollisionResponsetoChannel (Variables|Default|GetCapsuleComponent) "ECC_Pawn" "ECR_Ignore")
    (bind _asgame_mode_tecnocampus (Utilities|Casting|CastToGameModeTecnocampus (Game|GetGameMode)))
    (Default|IncrementScore _asgame_mode_tecnocampus 500)
    (Class|Pawn|DetachfromControllerPendingDestroy)
    (Utilities|FlowControl|Delay 3.0)
    (Actor|DestroyActor)))

(fn ConstructionScript
  (|CallParentFunction))